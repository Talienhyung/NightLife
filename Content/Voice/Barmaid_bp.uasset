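; Barmaid interactable that serves the player drinks, with voice lines.
; A box overlap toggles an indicator sphere and an in-range flag.
; Tick polls the character's PressE, latched to once per press, to play a sound, call Drinking on the character and count drinks.
; The second drink alone triggers a delayed extra line, with interaction locked until it finishes.
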(event `self.Box.OnComponentBeginOverlap`
  (params (OverlappedComponent :type "PrimitiveComponent Object Reference") (OtherActor :type "Actor Object Reference") (OtherComp :type "PrimitiveComponent Object Reference") (OtherBodyIndex :type Integer) (bFromSweep :type Boolean) (SweepResult :type "HitResult Structure (by ref)"))
  (bind _sphere (`self.Sphere`))
  (if (== OtherActor (`GameplayStatics.GetPlayerPawn` 0))
    (`SceneComponent.SetVisibility` _sphere true false)
    (set `self.InCollision` true)
    (else
      (`SceneComponent.SetVisibility` _sphere false false :!label _label)
      (set `self.InCollision` false))))

(event `self.Box.OnComponentEndOverlap`
  (params (OverlappedComponent :type "PrimitiveComponent Object Reference") (OtherActor :type "Actor Object Reference") (OtherComp :type "PrimitiveComponent Object Reference") (OtherBodyIndex :type Integer))
  (goto _label))

(event `self.ReceiveTick`
  (params (DeltaSeconds :type "Float (single-precision)"))
  (if (`self.stop`)
    _
    (elif (`self.InCollision`)
      (bind _asbp_third_person_character (cast `/Game/ThirdPerson/Blueprints/BP_ThirdPersonCharacter` (`GameplayStatics.GetPlayerCharacter` 0)))
      (if (`/Game/ThirdPerson/Blueprints/BP_ThirdPersonCharacter.pressE` _asbp_third_person_character)
        (if (not (`self.press`))
          (`GameplayStatics.PlaySound2D` "/Game/Voice/UNVERRE.UNVERRE" 1.0 1.0 0.0 null null)
          (set `self.press` true)
          (bind _asbp_third_person_character_2 (cast `/Game/ThirdPerson/Blueprints/BP_ThirdPersonCharacter` (`GameplayStatics.GetPlayerCharacter` 0)))
          (`/Game/ThirdPerson/Blueprints/BP_ThirdPersonCharacter.Drinking` _asbp_third_person_character_2)
          (set `self.Drink` (+ (`self.Drink`) 1))
          (if (== (`self.Drink`) 2)
            (set `self.stop` true)
            (`KismetSystemLibrary.Delay` 3.0)
            (`GameplayStatics.PlaySound2D` "/Game/Voice/demainjaicour.demainjaicour" 1.0 1.0 0.0 null null)
            (`KismetSystemLibrary.Delay` 6.0)
            (set `self.stop` false)))
        (else
          (set `self.press` false))))))

(fn `UserConstructionScript`)