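; RecalGurl is an interactable NPC who responds with voice lines and can reject the player.
; Box overlap toggles a sphere marker and enables Tick polling of the character's PressE.
; The Barmaid's Drink value selects either a "no guts" line (at zero) or a rejection sequence that calls AddRateau on FutureFemme only once.
; A Stop flag with Delays blocks retriggering during playback.
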(event `self.Box.OnComponentBeginOverlap`
  (params (OverlappedComponent :type "PrimitiveComponent Object Reference") (OtherActor :type "Actor Object Reference") (OtherComp :type "PrimitiveComponent Object Reference") (OtherBodyIndex :type Integer) (bFromSweep :type Boolean) (SweepResult :type "HitResult Structure (by ref)"))
  ;[1 1 1] Collision
  (if (== OtherActor (`GameplayStatics.GetPlayerPawn` 0))
    (`SceneComponent.SetVisibility` (`self.Sphere`) true false)
    (set `self.collli` true)))

(event `self.Box.OnComponentEndOverlap`
  (params (OverlappedComponent :type "PrimitiveComponent Object Reference") (OtherActor :type "Actor Object Reference") (OtherComp :type "PrimitiveComponent Object Reference") (OtherBodyIndex :type Integer))
  ;[1 1 1] Collision
  (`SceneComponent.SetVisibility` (`self.Sphere`) false false)
  (set `self.collli` false))

(event `self.ReceiveTick`
  (params (DeltaSeconds :type "Float (single-precision)"))
  (if (`self.stop`)
    _
    (elif (`self.collli`)
      (bind _asbp_third_person_character (cast `/Game/ThirdPerson/Blueprints/BP_ThirdPersonCharacter` (`GameplayStatics.GetPlayerPawn` 0)))
      (if (`/Game/ThirdPerson/Blueprints/BP_ThirdPersonCharacter.Press E` _asbp_third_person_character)
        (if (not (`self.press`))
          (bind _outactors (`GameplayStatics.GetAllActorsOfClass` "/Game/Voice/Barmaid_bp.Barmaid_bp_C"))
          (if (== (`/Game/Voice/Barmaid_bp.Drink` (`|GetArrayItem` _outactors)) 0)
            (`GameplayStatics.PlaySound2D` "/Game/Voice/PasLesCouilles.PasLesCouilles" 1.0 1.0 0.0 null null)
            (set `self.stop` true)
            (else
              (`GameplayStatics.PlaySound2D` "/Game/Voice/Dégage.Dégage" 1.0 1.0 0.0 null null)
              (set `self.stop` true)
              (`KismetSystemLibrary.Delay` 5.0)
              (`GameplayStatics.PlaySound2D` "/Game/Voice/REFOULE_.REFOULE_" 1.0 1.0 0.0 null null)
              (if (not (`self.rateau`))
                (bind _returnvalue (`GameplayStatics.GetActorOfClass` "/Game/Voice/FutureFemme_bp.FutureFemme_bp_C"))
                (`/Game/Voice/FutureFemme_bp.Add rateau` _returnvalue)
                (set `self.rateau` true))))
          (`KismetSystemLibrary.Delay` 5.0)
          (set `self.stop` false))
        (else
          (set `self.press` false))))))

(fn `UserConstructionScript`)