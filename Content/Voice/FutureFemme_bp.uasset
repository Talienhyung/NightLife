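; FutureFemme is an interactable NPC who plays voice lines and gives the player her number once a Rateau counter reaches two.
; Box overlap toggles a sphere indicator, and Tick polls the player character's PressE flag while in range.
; A high enough counter triggers a timed dialogue ending in GetNumber, otherwise another line plays, with a Stop flag providing cooldown.
; External events increment the counter or play a temporary hit-fall animation.
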(event `self.Box.OnComponentBeginOverlap`
  (params (OverlappedComponent :type "PrimitiveComponent Object Reference") (OtherActor :type "Actor Object Reference") (OtherComp :type "PrimitiveComponent Object Reference") (OtherBodyIndex :type Integer) (bFromSweep :type Boolean) (SweepResult :type "HitResult Structure (by ref)"))
  ;[1 1 1] Collision
  (if (== OtherActor (`GameplayStatics.GetPlayerPawn` 0))
    (`SceneComponent.SetVisibility` (`self.Sphere`) true false)
    (set `self.In Collision` true)))

(event `self.Box.OnComponentEndOverlap`
  (params (OverlappedComponent :type "PrimitiveComponent Object Reference") (OtherActor :type "Actor Object Reference") (OtherComp :type "PrimitiveComponent Object Reference") (OtherBodyIndex :type Integer))
  ;[1 1 1] Collision
  (`SceneComponent.SetVisibility` (`self.Sphere`) false false)
  (set `self.In Collision` false))

(event `self.ReceiveTick`
  (params (DeltaSeconds :type "Float (single-precision)"))
  (if (`self.stop`)
    _
    (elif (`self.In Collision`)
      (bind _asbp_third_person_character (cast `/Game/ThirdPerson/Blueprints/BP_ThirdPersonCharacter` (`GameplayStatics.GetPlayerCharacter` 0)))
      (if (`/Game/ThirdPerson/Blueprints/BP_ThirdPersonCharacter.Press E` _asbp_third_person_character)
        (if (not (`self.press`))
          (if (>= (`self.Rateau`) 2)
            (`GameplayStatics.PlaySound2D` "/Game/Voice/INVITATION_DANSE.INVITATION_DANSE" 1.0 1.0 0.0 null null)
            (set `self.stop` true)
            (`KismetSystemLibrary.Delay` 2.0)
            (`GameplayStatics.PlaySound2D` "/Game/Voice/NUMERO_DE_TELEPHONE.NUMERO_DE_TELEPHONE" 1.0 1.0 0.0 null null)
            (`KismetSystemLibrary.Delay` 6.0)
            (`GameplayStatics.PlaySound2D` "/Game/Voice/FIN.FIN" 1.0 1.0 0.0 null null)
            (bind _asbp_third_person_character_2 (cast `/Game/ThirdPerson/Blueprints/BP_ThirdPersonCharacter` (`GameplayStatics.GetPlayerCharacter` 0)))
            (`/Game/ThirdPerson/Blueprints/BP_ThirdPersonCharacter.Get Number` _asbp_third_person_character_2)
            (else
              (`GameplayStatics.PlaySound2D` "/Game/Voice/autre.autre" 1.0 1.0 0.0 null null)
              (set `self.stop` true)))
          (`KismetSystemLibrary.Delay` 10.0)
          (set `self.stop` false))
        (else
          (set `self.press` false))))))

(event `Add rateau`
  (set `self.Rateau` (+ (`self.Rateau`) 1)))

(event `BeingHit`
  (`SkeletalMeshComponent.PlayAnimation` (`self.Mesh`) "/Game/SCK_Casual01/Mannequin/Animations/HitFall.HitFall" false)
  (`KismetSystemLibrary.Delay` 2.0)
  (`SkeletalMeshComponent.SetAnimInstanceClass` (`self.Mesh`) "/Game/SCK_Casual01/Mannequin/Animations/ThirdPerson_AnimBP.ThirdPerson_AnimBP_C"))

(fn `UserConstructionScript`)